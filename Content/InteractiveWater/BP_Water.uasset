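; BP_Water is an interactive water surface that sends out a ripple where an actor enters its trigger.
; On BeginPlay it creates a dynamic material instance on WaterPlane.
; A WaterTrigger overlap writes the actor's location to RippleCenter and plays TL_Ripple, which drives the material's RippleRadius.
; The timeline uses Play rather than PlayFromStart, and the single center parameter supports one ripple at a time.
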(event OnComponentBeginOverlap(WaterTrigger)
  (params (OverlappedComponent :type Primitive%20Component%20Object%20Reference) (OtherActor :type Actor%20Object%20Reference) (OtherComp :type Primitive%20Component%20Object%20Reference) (OtherBodyIndex :type Integer) (bFromSweep :type Boolean) (SweepResult :type Hit%20Result%20Structure%20%28by%20ref%29))
  (Rendering|Material|SetVectorParameterValue (Variables|Default|GetWaterMID) "RippleCenter" (Math|Conversions|ToLinearColor(Vector) (Transformation|GetActorLocation OtherActor)) :!class /Script/Engine.MaterialInstanceDynamic)
  (bind _rippleradius (Timeline|TL_Ripple Play)
    (:Update
      (Rendering|Material|SetScalarParameterValue (Variables|Default|GetWaterMID) "RippleRadius" _rippleradius :!class /Script/Engine.MaterialInstanceDynamic))))

(event EventBeginPlay
  (bind _returnvalue (Rendering|Material|CreateDynamicMaterialInstance (Variables|Default|GetWaterPlane) 0 0 "None" :!class /Script/Engine.PrimitiveComponent))
  (Variables|Default|SetWaterMID _returnvalue))

(fn ConstructionScript)